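; BP_FollowScript is an actor that trails the side-scroller player along the Y axis, moving whenever the gap exceeds a trigger distance.
; BeginPlay caches the controlled pawn, and CheckDistancePlayer measures the absolute Y gap to set the Moving flag.
; While moving, Tick rechecks and adds a fixed per-frame Y offset, independent of player side and delta time.
; While idle, it rechecks through a 0.2-second Delay.
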(event Custom|UpdateFollowing
  (bind _distancefromplayer (CallFunction|CheckDistancePlayer))
  (if (> _distancefromplayer (Variables|Default|GetTriggerDistance))
    (Variables|Default|SetMoving true)
    (else
      (Variables|Default|SetMoving false))))

(event EventBeginPlay
  (bind _asbp_player_side_scroller (Utilities|Casting|CastToBP_PlayerSideScroller (Pawn|GetControlledPawn (Game|GetPlayerController 0))))
  (Variables|Default|SetPlayerReference _asbp_player_side_scroller))

(event EventTick
  (params (DeltaSeconds :type Float%20%28single-precision%29))
  (if (Variables|Default|GetMoving)
    (CallFunction|UpdateFollowing)
    (Transformation|AddActorWorldOffset (Math|Vector|MakeVector 0.0 (Variables|Default|GetActorMovingSpeed) 0.0))
    (else
      (Utilities|FlowControl|Sequence
        (:then_0
          (Utilities|FlowControl|Delay 0.2)
          (CallFunction|UpdateFollowing))))))

(fn ConstructionScript)

(fn CheckDistancePlayer
  (bind _returnvalue (Transformation|GetActorLocation))
  (bind _playerreference (Variables|Default|GetPlayerReference))
  (bind _returnvalue_2 (Transformation|GetActorLocation _playerreference))
  (if (> (.y _returnvalue_2) (.y _returnvalue))
    (bind _output_get (LocalVariables|SetDistance (- (.y _returnvalue_2) (.y _returnvalue))))
    (return _output_get)
    (else
      (bind _output_get_2 (LocalVariables|SetDistance (- (.y _returnvalue) (.y _returnvalue_2))))
      (return _output_get_2))))
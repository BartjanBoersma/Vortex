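; Player controller for the side-scroller character, turning input into ability actions gated by boolean flags.
; On BeginPlay it caches BP_PlayerSideScroller, which holds most state the abilities change.
; True Vision toggles aura platform visibility and collision with a cooldown; sprint rescales the player's Duration; double jump uses a DoN reset on landing.
; Pickup line-traces into a physics handle, Interact spawns melee particles and opens doors, and shooting is a stub.
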(event Custom|ShootEvent
  (if (Variables|Abilities|GetShootAbility)
    _))

(event Custom|JumpEvent
  ;[1 1 1] Jump Ability
  (if (Variables|Abilities|GetJumpAbility)
    (if (Variables|Abilities|GetDoubleJumpAbility)
      (bind _counter (Utilities|FlowControl|DoN 2)
        (:Exit
          (switch int _counter
            (:1
              (Character|Jump (Variables|Default|GetPlayerRef)))
            (:2
              (Character|LaunchCharacter (Variables|Default|GetPlayerRef) "0, 0,600.000000" false false)))))
      (else
        (Character|Jump (Variables|Default|GetPlayerRef))))))

(event Custom|Drop
  (bind _playerref (Variables|Default|GetPlayerRef))
  (bind _physicsobject (Variables|/Game/VortexGame/Core/BP_PlayerSideScroller.BP_PlayerSideScroller_C|GetPhysicsObject _playerref))
  ;[1 1 1] Pick Up Ability
  (Physics|Components|PhysicsHandle|ReleaseComponent (Variables|/Game/VortexGame/Core/BP_PlayerSideScroller.BP_PlayerSideScroller_C|GetPhysicsHandle (Variables|Default|GetPlayerRef)))
  (Variables|/Game/VortexGame/Core/BP_PlayerSideScroller.BP_PlayerSideScroller_C|SetIsHoldingObject (Variables|Default|GetPlayerRef) false)
  (Collision|SetCollisionResponsetoChannel _physicsobject "ECC_Pawn" "ECR_Block")
  (Class|PrimitiveComponent|SetAllPhysicsLinearVelocity _physicsobject "0, 0, 0" false)
  (Utilities|FlowControl|Delay 0.2)
  (Class|PrimitiveComponent|SetAngularDamping _physicsobject 0.0))

(event Custom|PickUpEvent
  (bind _playerref (Variables|Default|GetPlayerRef))
  (bind _playerref_2 (Variables|Default|GetPlayerRef))
  (bind _playerref_3 (Variables|Default|GetPlayerRef))
  (bind _rotationcomponent (Variables|/Game/VortexGame/Core/BP_PlayerSideScroller.BP_PlayerSideScroller_C|GetRotationComponent _playerref_3))
  (bind _returnvalue (Transformation|GetWorldLocation _rotationcomponent))
  ;[1 1 1] Pick Up Ability
  (if (Variables|Abilities|GetPickUpAbility)
    (bind (_outhit _returnvalue_2) (Collision|LineTraceForObjects _returnvalue (+ _returnvalue (* (Math|Vector|GetForwardVector _rotationcomponent) 5e+02)) (Utilities|Array|MakeArray "ObjectTypeQuery4") false 0 "Persistent"))
    (if _returnvalue_2
      (Variables|/Game/VortexGame/Core/BP_PlayerSideScroller.BP_PlayerSideScroller_C|SetPhysicsObject _playerref (.HitComponent (Collision|BreakHitResult _outhit)))
      (Class|PhysicsHandleComponent|GrabComponentatLocation (Variables|/Game/VortexGame/Core/BP_PlayerSideScroller.BP_PlayerSideScroller_C|GetPhysicsHandle _playerref) (.HitComponent (Collision|BreakHitResult _outhit)) "None" (.Location (Collision|BreakHitResult _outhit)))
      (Variables|/Game/VortexGame/Core/BP_PlayerSideScroller.BP_PlayerSideScroller_C|SetIsHoldingObject _playerref_2 true)
      (Collision|SetCollisionResponsetoChannel (Variables|/Game/VortexGame/Core/BP_PlayerSideScroller.BP_PlayerSideScroller_C|GetPhysicsObject _playerref_2) "ECC_Pawn" "ECR_Ignore"))))

(event Custom|EventOnLanded
  ;[1 1 1] Jump Ability
  (Utilities|FlowControl|DoN 2) ; enters at Reset
)

(event Custom|MeleeAttackEvent
  (bind _playerref (Variables|Default|GetPlayerRef))
  (bind _particleeffect (Variables|/Game/VortexGame/Core/BP_PlayerSideScroller.BP_PlayerSideScroller_C|GetParticleEffect _playerref))
  (bind _returnvalue (Transformation|GetWorldTransform _particleeffect))
  (if (Variables|Abilities|GetMeleeAttackAbility)
    (Effects|SpawnEmitteratLocation "/Game/VortexGame/Effects/P_Melee_Attack.P_Melee_Attack" (.location _returnvalue) (.rotation _returnvalue) "3.000000,3.000000,3.000000")))

(event Custom|SprintEvent_Pressed
  (bind _playerref (Variables|Default|GetPlayerRef))
  (Variables|/Game/VortexGame/Core/BP_PlayerSideScroller.BP_PlayerSideScroller_C|SetDuration (Variables|Default|GetPlayerRef) (/ (Variables|/Game/VortexGame/Core/BP_PlayerSideScroller.BP_PlayerSideScroller_C|GetDefaultRadiusCurrentLevel _playerref) (Variables|/Game/VortexGame/Core/BP_PlayerSideScroller.BP_PlayerSideScroller_C|GetSprintSpeedMultiplier _playerref))))

(event Custom|SprintEvent_Released
  (bind _playerref (Variables|Default|GetPlayerRef))
  (Variables|/Game/VortexGame/Core/BP_PlayerSideScroller.BP_PlayerSideScroller_C|SetDuration _playerref (Variables|/Game/VortexGame/Core/BP_PlayerSideScroller.BP_PlayerSideScroller_C|GetDefaultRadiusCurrentLevel _playerref)))

(event Custom|EnableHighJumpEvent
  (Variables|Abilities|SetHighJumpAbiltiy true)
  (Variables|/Script/Engine.CharacterMovementComponent|SetJumpZVelocity (Variables|/Script/Engine.Character|GetCharacterMovement (Variables|Default|GetPlayerRef)) 9e+02))

(event Custom|TrueVisionEvent
  (bind _playerref (Variables|Default|GetPlayerRef))
  (bind _playerref_2 (Variables|Default|GetPlayerRef))
  (bind _auraplatformsreference (Variables|/Game/VortexGame/Core/BP_PlayerSideScroller.BP_PlayerSideScroller_C|GetAuraPlatformsReference _playerref))
  (bind _truevisioncooldown (Variables|/Game/VortexGame/Core/BP_PlayerSideScroller.BP_PlayerSideScroller_C|GetTrueVisionCooldown _playerref_2))
  ;[0 1 0.9345] Truevision Functionality
  (if (Variables|Abilities|GetTrueVision)
    (if (not (AI|Components|NavMovement|IsFalling (Variables|/Script/Engine.Character|GetCharacterMovement (Variables|Default|GetPlayerRef))))
      (if (not (Variables|/Game/VortexGame/Core/BP_PlayerSideScroller.BP_PlayerSideScroller_C|GetWasTrueVisionJustActivated (Variables|Default|GetPlayerRef)))
        (Utilities|FlowControl|FlipFlop
          (:A
            (for _array_element _auraplatformsreference
              (Rendering|SetVisibility (Variables|/Game/VortexGame/Core/Interactables/AuraObjects/BP_AuraPlatform.BP_AuraPlatform_C|GetCubeforingame _array_element) true false)
              (Collision|SetCollisionEnabled (Variables|/Game/VortexGame/Core/Interactables/AuraObjects/BP_AuraPlatform.BP_AuraPlatform_C|GetCubeforingame _array_element) "QueryAndPhysics")
              (Variables|/Game/VortexGame/Core/BP_PlayerSideScroller.BP_PlayerSideScroller_C|SetWasTrueVisionJustActivated (Variables|Default|GetPlayerRef) true)
              (Utilities|FlowControl|Delay _truevisioncooldown)
              (Variables|/Game/VortexGame/Core/BP_PlayerSideScroller.BP_PlayerSideScroller_C|SetWasTrueVisionJustActivated (Variables|Default|GetPlayerRef) false)))
          (:B
            (for _array_element_2 _auraplatformsreference
              (Rendering|SetVisibility (Variables|/Game/VortexGame/Core/Interactables/AuraObjects/BP_AuraPlatform.BP_AuraPlatform_C|GetCubeforingame _array_element_2) false false)
              (Collision|SetCollisionEnabled (Variables|/Game/VortexGame/Core/Interactables/AuraObjects/BP_AuraPlatform.BP_AuraPlatform_C|GetCubeforingame _array_element_2) "NoCollision")
              (Variables|/Game/VortexGame/Core/BP_PlayerSideScroller.BP_PlayerSideScroller_C|SetWasTrueVisionJustActivated (Variables|Default|GetPlayerRef) true)
              (Utilities|FlowControl|Delay _truevisioncooldown)
              (Variables|/Game/VortexGame/Core/BP_PlayerSideScroller.BP_PlayerSideScroller_C|SetWasTrueVisionJustActivated (Variables|Default|GetPlayerRef) false))))))))

(event EventBeginPlay
  (bind _asbp_player_side_scroller (Utilities|Casting|CastToBP_PlayerSideScroller (Pawn|GetControlledPawn)))
  (Variables|Default|SetPlayerRef _asbp_player_side_scroller))

(event Input|ActionEvents|InputActionInteract
  (params (Key :type Key%20Structure))
  (bind _playerref (Variables|Default|GetPlayerRef))
  (bind _doorinteractable (Variables|/Game/VortexGame/Core/BP_PlayerSideScroller.BP_PlayerSideScroller_C|GetDoorInteractable _playerref))
  (:Pressed
    (CallFunction|MeleeAttackEvent)
    (Utilities|IsValid _doorinteractable
      (:Is%20Valid
        (Variables|/Game/VortexGame/Core/Interactables/House/BP_OpenDoor.BP_OpenDoor_C|SetOpen _doorinteractable true)))))

(event Input|ActionEvents|InputActionChangeVision1
  (params (Key :type Key%20Structure))
  (:Pressed
    (CallFunction|TrueVisionEvent)))

(event Input|ActionEvents|InputActionJump
  (params (Key :type Key%20Structure))
  (:Pressed
    (CallFunction|JumpEvent)))

(event Input|ActionEvents|InputActionSprint
  (params (Key :type Key%20Structure))
  (:Pressed
    (if (Variables|Abilities|GetSprintAbility)
      (CallFunction|SprintEventPressed)))
  (:Released
    (CallFunction|SprintEventReleased)))

(event Input|ActionEvents|InputActionAction
  (params (Key :type Key%20Structure))
  (bind _pickupability (Variables|Abilities|GetPickUpAbility))
  (:Pressed
    (Utilities|FlowControl|DoOnce false :!label _label
      (:Completed
        (Utilities|FlowControl|FlipFlop
          (:A
            (if _pickupability
              (CallFunction|PickUpEvent)))
          (:B
            (if _pickupability
              (CallFunction|Drop)))))))
  (:Released
    (goto _label Reset)))

(fn ConstructionScript)
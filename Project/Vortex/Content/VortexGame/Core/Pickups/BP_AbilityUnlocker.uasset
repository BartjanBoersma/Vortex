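; BP_AbilityUnlocker is a pickup that sells the player one ability, chosen by its Ability enum, for a Price in Money.
; On any actor overlap it fetches player 0's controller and side-scroller pawn, without checking what overlapped.
; With enough Money, it deducts the price, sets the matching controller flag, prints the unlock and destroys itself; otherwise it prints a refusal.
; The construction script applies UnlockMesh to the static mesh.
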(event EventBeginPlay)

(event Collision|EventActorBeginOverlap
  (params (OtherActor :type Actor%20Object%20Reference))
  (bind _asbp_player_controller (Utilities|Casting|CastToBP_PlayerController (Game|GetPlayerController 0)))
  (Variables|Default|SetPlayerController _asbp_player_controller)
  (bind _asbp_player_side_scroller (Utilities|Casting|CastToBP_PlayerSideScroller (Game|Player|GetPlayerPawn 0)))
  (bind _output_get (Variables|Default|SetPlayerRef _asbp_player_side_scroller))
  (if (>= (Variables|/Game/VortexGame/Core/BP_PlayerSideScroller.BP_PlayerSideScroller_C|GetMoney _output_get) (Variables|Unlocking|GetPrice))
    (Variables|/Game/VortexGame/Core/BP_PlayerSideScroller.BP_PlayerSideScroller_C|SetMoney (Variables|Default|GetPlayerRef) (- (Variables|/Game/VortexGame/Core/BP_PlayerSideScroller.BP_PlayerSideScroller_C|GetMoney (Variables|Default|GetPlayerRef)) (Variables|Unlocking|GetPrice)))
    (switch Utilities|FlowControl|Switch|SwitchonEAbilities (Variables|Unlocking|GetAbility)
      (:NewEnumerator0
        (Variables|/Game/VortexGame/Core/BP_PlayerController.BP_PlayerController_C|SetJumpAbility (Variables|Default|GetPlayerController) true))
      (:NewEnumerator1
        (Variables|/Game/VortexGame/Core/BP_PlayerController.BP_PlayerController_C|SetShootAbility (Variables|Default|GetPlayerController) true))
      (:NewEnumerator2
        (Variables|/Game/VortexGame/Core/BP_PlayerController.BP_PlayerController_C|SetPickUpAbility (Variables|Default|GetPlayerController) true))
      (:NewEnumerator3
        (Variables|/Game/VortexGame/Core/BP_PlayerController.BP_PlayerController_C|SetDoubleJumpAbility (Variables|Default|GetPlayerController) true))
      (:NewEnumerator4
        (Variables|/Game/VortexGame/Core/BP_PlayerController.BP_PlayerController_C|SetSprintAbility (Variables|Default|GetPlayerController) true))
      (:NewEnumerator5
        (Variables|/Game/VortexGame/Core/BP_PlayerController.BP_PlayerController_C|SetHighJumpAbiltiy (Variables|Default|GetPlayerController) true))
      (:NewEnumerator6
        (Variables|/Game/VortexGame/Core/BP_PlayerController.BP_PlayerController_C|SetMeleeAttackAbility (Variables|Default|GetPlayerController) true))
      (:NewEnumerator7
        (Variables|/Game/VortexGame/Core/BP_PlayerController.BP_PlayerController_C|SetRangedAttackAbility (Variables|Default|GetPlayerController) true)))
    (Development|PrintString (Utilities|String|Append "You Unlocked" (Utilities|String|EnumtoString (Variables|Unlocking|GetAbility))))
    (Actor|DestroyActor)
    (else
      (Development|PrintString "Not Enough Money"))))

(fn ConstructionScript
  (Components|StaticMesh|SetStaticMesh (Variables|Components|GetStaticMesh) (Variables|Unlocking|GetUnlockMesh)))
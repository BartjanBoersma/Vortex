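; Toy pickup for the side-scroller that adds its Worth to the player's Money.
; BeginPlay caches the player pawn; when the Box is overlapped by a BP_PlayerSideScroller while Enabled, the new total is written to it and printed.
; The pickup neither disables nor destroys itself in these graphs.
; ChangeMesh picks a random mesh from MeshArray but is never called here, and its maximum index overruns the array by one.
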(event OnComponentBeginOverlap(Box)
  (params (OverlappedComponent :type Primitive%20Component%20Object%20Reference) (OtherActor :type Actor%20Object%20Reference) (OtherComp :type Primitive%20Component%20Object%20Reference) (OtherBodyIndex :type Integer) (bFromSweep :type Boolean) (SweepResult :type Hit%20Result%20Structure%20%28by%20ref%29))
  (if (Variables|Default|GetbEnabled?)
    (bind _asbp_player_side_scroller (Utilities|Casting|CastToBP_PlayerSideScroller OtherActor))
    (bind _output_get (Variables|/Game/VortexGame/Core/BP_PlayerSideScroller.BP_PlayerSideScroller_C|SetMoney (Variables|Default|GetPlayerPawn) (+ (Variables|/Game/VortexGame/Core/BP_PlayerSideScroller.BP_PlayerSideScroller_C|GetMoney _asbp_player_side_scroller) (Variables|Components|GetWorth))))
    (Development|PrintString (Utilities|String|ToString(Integer) _output_get))))

(event EventBeginPlay
  (bind _asbp_player_side_scroller (Utilities|Casting|CastToBP_PlayerSideScroller (Game|Player|GetPlayerPawn 0)))
  (Variables|Default|SetPlayerPawn _asbp_player_side_scroller))

(event EventTick
  (params (DeltaSeconds :type Float%20%28single-precision%29)))

(fn ConstructionScript)

(fn ChangeMesh
  (bind _mesharray (Variables|Default|GetMeshArray))
  (Components|StaticMesh|SetStaticMesh (Variables|Default|GetStaticMesh) (Utilities|Array|Get(acopy) _mesharray (Math|Random|RandomIntegerinRange 0 (Utilities|Array|Length _mesharray)))))
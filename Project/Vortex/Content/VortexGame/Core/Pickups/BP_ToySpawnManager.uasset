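; Manager that randomly chooses which placed toy pickups are active in each round.
; Construction script caches every BP_ToyPickup in AllPickups, and RoundUpdated stores the round and calls RefreshPoints.
; RefreshPoints disables and hides all pickups, then enables and shows random picks, looping by that level's SGameBalance toy count.
; Picks use AddUnique with an upper index of array length, so duplicates or an out-of-range index can skew the count.
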(event Custom|RoundUpdated
  (params (Roundnr :type Integer))
  (Variables|Default|SetCurrentRound Roundnr)
  (CallFunction|RefreshPoints))

(event EventBeginPlay)

(event Collision|EventActorBeginOverlap
  (params (OtherActor :type Actor%20Object%20Reference)))

(event EventTick
  (params (DeltaSeconds :type Float%20%28single-precision%29)))

(fn ConstructionScript
  (bind _outactors (Actor|GetAllActorsOfClass "/Game/VortexGame/Core/Pickups/BP_ToyPickup.BP_ToyPickup_C"))
  (Variables|Default|SetAllPickups _outactors))

(fn RefreshPoints
  (bind _sgamebalance (Variables|Default|GetSGameBalance))
  (bind _allpickups (Variables|Default|GetAllPickups))
  (for _array_element (Variables|Default|GetAllPickups)
    (Variables|/Game/VortexGame/Core/Pickups/BP_ToyPickup.BP_ToyPickup_C|SetbEnabled? _array_element false)
    (Rendering|SetVisibility (Variables|/Script/Engine.Actor|GetRootComponent _array_element) false false)
    (Rendering|SetActorHiddenInGame _array_element true))
  (Utilities|Array|Clear (Variables|Default|GetAvailablePickups))
  (for _index (range 0 (.amountoftoypickups (Utilities|Select :Index (Variables|Default|GetCurrentRound) :Option%200 (.level1 _sgamebalance) :Option%201 (.level2 _sgamebalance) :Option%202 (.level3 _sgamebalance) :Option%203 (.level4 _sgamebalance) :Option%204 (.level5 _sgamebalance))))
    (Utilities|Array|AddUnique (Variables|Default|GetAvailablePickups) (Utilities|Array|Get(acopy) _allpickups (Math|Random|RandomIntegerinRange 0 (Utilities|Array|Length _allpickups)))))
  (for _array_element_2 (Variables|Default|GetAvailablePickups)
    (Variables|/Game/VortexGame/Core/Pickups/BP_ToyPickup.BP_ToyPickup_C|SetbEnabled? _array_element_2 true)
    (Rendering|SetVisibility (Variables|/Script/Engine.Actor|GetRootComponent _array_element_2) true true)
    (Rendering|SetActorHiddenInGame _array_element_2 false)))
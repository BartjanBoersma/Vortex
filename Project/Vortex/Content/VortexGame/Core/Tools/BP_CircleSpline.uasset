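; Editor-placeable tool actor that builds a four-point spline intended as a circle, sized by Radius.
; The construction script clears the spline and adds points on the local X and Y axes, with Offset scaling the opposite pair.
; It then sets Y-only tangents per point, alternating positive, zero, negative and zero, scaled from the Bezier circle constant 4(√2−1)/3.
; Event graph logic is empty.
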(event EventBeginPlay
  (|CallParentFunction) ; This node is disabled and will not be called.\nDrag off pins to build functionality.
)

(event Collision|EventActorBeginOverlap
  (params (OtherActor :type Actor%20Object%20Reference))
  (|CallParentFunction OtherActor) ; This node is disabled and will not be called.\nDrag off pins to build functionality.
)

(event EventTick
  (params (DeltaSeconds :type Float%20%28single-precision%29))
  (|CallParentFunction DeltaSeconds) ; This node is disabled and will not be called.\nDrag off pins to build functionality.
)

(fn ConstructionScript
  (bind _radius (Variables|Default|GetRadius))
  (bind _radius_2 (Variables|Default|GetRadius))
  (|CallParentFunction)
  (Spline|ClearSplinePoints (Variables|Default|GetSpline) true)
  (Spline|AddSplinePoint (Variables|Default|GetSpline) (Math|Vector|MakeVector _radius 0.0 0.0) "Local" true)
  (Spline|AddSplinePoint (Variables|Default|GetSpline) (Math|Vector|MakeVector 0.0 _radius 0.0) "Local" true)
  (Spline|AddSplinePoint (Variables|Default|GetSpline) (Math|Vector|MakeVector (* _radius_2 (Variables|Default|GetOffset)) 0.0 0.0) "Local" true)
  (Spline|AddSplinePoint (Variables|Default|GetSpline) (Math|Vector|MakeVector 0.0 (* _radius_2 (Variables|Default|GetOffset)) 0.0) "Local" true)
  (for _index (range 0 (Spline|GetNumberOfSplinePoints (Variables|Default|GetSpline)))
    (bind _output_get (Variables|Default|SetSplineNum _index))
    (if (== _output_get 0)
      (CallFunction|SetTangentatSplinePoint 1.0)
      (elif (== (Variables|Default|GetSplineNum) 1)
        (CallFunction|SetTangentatSplinePoint 0.0)
        (elif (== (Variables|Default|GetSplineNum) 2)
          (CallFunction|SetTangentatSplinePoint -1.0)
          (elif (== (Variables|Default|GetSplineNum) 3)
            (CallFunction|SetTangentatSplinePoint 0.0)))))))

(fn SetTangentatSplinePoint
  (params (VariableFloat :type Float%20%28single-precision%29))
  (Spline|SetTangentatSplinePoint (Variables|Default|GetSpline) (Variables|Default|GetSplineNum) (Math|Vector|MakeVector 0.0 (* (* (Variables|Default|GetRadius) (+ (|((4*((sqrt(2))-1))/3)) 1.0)) VariableFloat) 0.0) "Local" true))
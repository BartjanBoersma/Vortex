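; BP_UpdateRound is a trigger actor that advances the Round counter on GM_MetroidVania as the side-scroller player passes through it.
; When the player stops overlapping Entry while CanIncremment is set, it increments the game mode's Round, copies it to CurrentRound and clears the flag.
; Leaving Exit sets the flag again, a latch that prevents repeated Entry crossings from counting extra rounds.
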(event OnComponentEndOverlap(Exit)
  (params (OverlappedComponent :type Primitive%20Component%20Object%20Reference) (OtherActor :type Actor%20Object%20Reference) (OtherComp :type Primitive%20Component%20Object%20Reference) (OtherBodyIndex :type Integer))
  (Utilities|Casting|CastToBP_PlayerSideScroller OtherActor)
  (Variables|Default|SetCanIncremment true))

(event OnComponentEndOverlap(Entry)
  (params (OverlappedComponent :type Primitive%20Component%20Object%20Reference) (OtherActor :type Actor%20Object%20Reference) (OtherComp :type Primitive%20Component%20Object%20Reference) (OtherBodyIndex :type Integer))
  (Utilities|Casting|CastToBP_PlayerSideScroller OtherActor)
  (bind _asgm_metroid_vania (Utilities|Casting|CastToGM_MetroidVania (Game|GetGameMode)))
  (if (Variables|Default|GetCanIncremment)
    (bind _result (Math|Integer|IncrementInt (Variables|/Game/VortexGame/Core/GameModes/GM_MetroidVania.GM_MetroidVania_C|GetRound _asgm_metroid_vania))
      (:%20%20
        (Variables|Default|SetCurrentRound _result)
        (Variables|Default|SetCanIncremment false)))))

(event EventBeginPlay)

(event Collision|EventActorBeginOverlap
  (params (OtherActor :type Actor%20Object%20Reference)))

(event EventTick
  (params (DeltaSeconds :type Float%20%28single-precision%29)))

(fn ConstructionScript)
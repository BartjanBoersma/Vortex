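; Enemy spawner actor that spawns BP_BaseEnemy at its own transform, capped per round by GameBalance.
; Tick runs through a two-second Delay as a repeating timer, then switches on GM_MetroidVania's Round across five levels.
; Each round's DoN gate limits spawns to that level's enemy count.
; Spawned enemies receive movement and patrol splines and a duration, set their spline timeline to 1.0 and start moving in reverse.
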(event EventTick
  (params (DeltaSeconds :type Float%20%28single-precision%29))
  (bind _gamebalance (Variables|Default|GetGameBalance))
  (bind _asgm_metroid_vania (Utilities|Casting|CastToGM_MetroidVania (Game|GetGameMode)))
  (Utilities|FlowControl|Delay 2.0)
  (switch int (Variables|/Game/VortexGame/Core/GameModes/GM_MetroidVania.GM_MetroidVania_C|GetRound _asgm_metroid_vania)
    (:0
      (Utilities|FlowControl|DoN (.amountofenemies (.level1 _gamebalance))
        (:Exit
          _)))
    (:1
      (Utilities|FlowControl|DoN (.amountofenemies (.level2 _gamebalance))
        (:Exit
          _)))
    (:2
      (Utilities|FlowControl|DoN (.amountofenemies (.level3 _gamebalance))
        (:Exit
          _)))
    (:3
      (Utilities|FlowControl|DoN (.amountofenemies (.level4 _gamebalance))
        (:Exit
          _)))
    (:4
      (Utilities|FlowControl|DoN (.amountofenemies (.level5 _gamebalance))
        (:Exit
          _))))
  (bind _returnvalue (Game|SpawnActorfromClass "/Game/VortexGame/Core/Interactables/BP_BaseEnemy.BP_BaseEnemy_C" (Transformation|GetWorldTransform (Variables|Default|GetDefaultSceneRoot)) "Undefined" 0 0))
  (Variables|/Game/VortexGame/Core/Tools/BP_MoveAlongSpline.BP_MoveAlongSpline_C|SetMovementSpline _returnvalue (Variables|Default|GetSpawnSpline))
  (Variables|/Game/VortexGame/Core/Interactables/BP_BaseEnemy.BP_BaseEnemy_C|SetPatrolSpline _returnvalue (Variables|Default|GetPatrolSpline))
  (Variables|/Game/VortexGame/Core/Tools/BP_MoveAlongSpline.BP_MoveAlongSpline_C|SetDuration _returnvalue (Variables|Default|GetMovementDuration))
  (Components|Timeline|SetNewTime (Variables|/Game/VortexGame/Core/Tools/BP_MoveAlongSpline.BP_MoveAlongSpline_C|GetMoveAlongSpline_TL _returnvalue) 1.0)
  (Default|MoveReverse _returnvalue))

(fn ConstructionScript)
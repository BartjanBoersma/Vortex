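; BP_FallingRails is a length-configurable stretch of train track that collapses after the side-scroller player passes its end.
; The construction script lays out LengthCount track meshes along Y after the base RailMesh, collects them in Rails, and adds a box, EndCollision, at the far end.
; When BP_PlayerSideScroller stops overlapping that box, every rail starts simulating physics at once.
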(event OnComponentEndOverlap(EndCollision)
  (params (OverlappedComponent :type Primitive%20Component%20Object%20Reference) (OtherActor :type Actor%20Object%20Reference) (OtherComp :type Primitive%20Component%20Object%20Reference) (OtherBodyIndex :type Integer))
  (Utilities|Casting|CastToBP_PlayerSideScroller OtherActor)
  (for _array_element (Variables|Default|GetRails)
    (Physics|SetSimulatePhysics _array_element true)))

(event EventBeginPlay)

(event Collision|EventActorBeginOverlap
  (params (OtherActor :type Actor%20Object%20Reference)))

(event EventTick
  (params (DeltaSeconds :type Float%20%28single-precision%29)))

(fn ConstructionScript
  (bind _rails (Variables|Default|GetRails))
  (bind _lengthcount (Variables|Default|GetLengthCount))
  (Utilities|Array|Clear _rails)
  (Utilities|Array|Add _rails (Variables|Default|GetRailMesh))
  (for _index (range 1 _lengthcount)
    (bind _returnvalue (AddComponent|AddStaticMeshComponent false (Math|Transform|MakeTransform (Math|Vector|MakeVector 0.0 (* _index 1e+02) 0.0) "0, 0, 0" "1,1,1")))
    (Components|StaticMesh|SetStaticMesh _returnvalue "/Game/VortexGame/Art/Nature/splineTrainTracks/SM_TrainTracks_trainTracks2.SM_TrainTracks_trainTracks2")
    (Utilities|Array|Add (Variables|Default|GetRails) _returnvalue))
  (bind _returnvalue_2 (AddComponent|AddBoxComponent false (Math|Transform|MakeTransform (Math|Vector|MakeVector 0.0 (+ (* _lengthcount 1e+02) 5e+01) 5e+01) "0, 0, 0" "1,1,1")))
  (Variables|Default|SetEndCollision _returnvalue_2))
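; Ability shop actor that sells player abilities for money when the side-scroller pawn overlaps one of three option triggers.
; BeginPlay maps four abilities to their unowned state, then labels three planes with materials from the first three AvailableAbilityNames, independent of that map.
; Overlap removes the option's map entry, then SetAbility checks Money against Price, deducts it and sets the controller's ability flag.
; An older enum-based purchase path remains unreachable.
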(event OnComponentBeginOverlap(Option_3)
  (params (OverlappedComponent :type Primitive%20Component%20Object%20Reference) (OtherActor :type Actor%20Object%20Reference) (OtherComp :type Primitive%20Component%20Object%20Reference) (OtherBodyIndex :type Integer) (bFromSweep :type Boolean) (SweepResult :type Hit%20Result%20Structure%20%28by%20ref%29))
  (bind _abilitynameoption_2 (Variables|Default|GetAbilityNameOption_2))
  (Utilities|Casting|CastToBP_PlayerSideScroller OtherActor)
  (Utilities|Map|Remove (Variables|Default|GetAvailableAbilities) _abilitynameoption_2)
  (CallFunction|SetAbility _abilitynameoption_2))

(event OnComponentBeginOverlap(Option_2)
  (params (OverlappedComponent :type Primitive%20Component%20Object%20Reference) (OtherActor :type Actor%20Object%20Reference) (OtherComp :type Primitive%20Component%20Object%20Reference) (OtherBodyIndex :type Integer) (bFromSweep :type Boolean) (SweepResult :type Hit%20Result%20Structure%20%28by%20ref%29))
  (bind _abilitynameoption_3 (Variables|Default|GetAbilityNameOption_3))
  (Utilities|Casting|CastToBP_PlayerSideScroller OtherActor)
  (Utilities|Map|Remove (Variables|Default|GetAvailableAbilities) _abilitynameoption_3)
  (CallFunction|SetAbility _abilitynameoption_3))

(event OnComponentBeginOverlap(Option_1)
  (params (OverlappedComponent :type Primitive%20Component%20Object%20Reference) (OtherActor :type Actor%20Object%20Reference) (OtherComp :type Primitive%20Component%20Object%20Reference) (OtherBodyIndex :type Integer) (bFromSweep :type Boolean) (SweepResult :type Hit%20Result%20Structure%20%28by%20ref%29))
  (bind _abilitynameoption_1 (Variables|Default|GetAbilityNameOption_1))
  (Utilities|Casting|CastToBP_PlayerSideScroller OtherActor)
  (Utilities|Map|Remove (Variables|Default|GetAvailableAbilities) _abilitynameoption_1)
  (CallFunction|SetAbility _abilitynameoption_1))

(event Custom|SetMaterials1stRound
  (bind _availableabilitynames (Variables|Default|GetAvailableAbilityNames))
  (bind _availableabilitynames_2 (Variables|Default|GetAvailableAbilityNames))
  (bind _availableabilitynames_3 (Variables|Default|GetAvailableAbilityNames))
  (bind _output (Utilities|Array|Get(acopy) _availableabilitynames 2))
  (bind _output_2 (Utilities|Array|Get(acopy) _availableabilitynames_2))
  (bind _output_3 (Utilities|Array|Get(acopy) _availableabilitynames_3 1))
  (CallFunction|SetMaterial (Variables|Default|GetPlane) _output_2)
  (Variables|Default|SetAbilityNameOption_1 _output_2)
  (CallFunction|SetMaterial (Variables|Default|Getplane1) _output_3)
  (Variables|Default|SetAbilityNameOption_2 _output_3)
  (CallFunction|SetMaterial (Variables|Default|Getplane2) _output)
  (Variables|Default|SetAbilityNameOption_3 _output))

(event EventBeginPlay
  (bind _availableabilities (Variables|Default|GetAvailableAbilities))
  (bind _asbp_player_controller (Utilities|Casting|CastToBP_PlayerController (Game|GetPlayerController 0)))
  (Variables|Default|SetPlayerRef _asbp_player_controller)
  (Utilities|Map|Add _availableabilities "JumpAbility" (not (Variables|/Game/VortexGame/Core/BP_PlayerController.BP_PlayerController_C|GetJumpAbility _asbp_player_controller)))
  (Utilities|Map|Add _availableabilities "MeleeAttackAbility" (not (Variables|/Game/VortexGame/Core/BP_PlayerController.BP_PlayerController_C|GetMeleeAttackAbility _asbp_player_controller)))
  (Utilities|Map|Add _availableabilities "DoubleJumpAbility" (not (Variables|/Game/VortexGame/Core/BP_PlayerController.BP_PlayerController_C|GetDoubleJumpAbility _asbp_player_controller)))
  (Utilities|Map|Add _availableabilities "SprintAbility" (not (Variables|/Game/VortexGame/Core/BP_PlayerController.BP_PlayerController_C|GetSprintAbility _asbp_player_controller)))
  (CallFunction|SetMaterials1stRound))

(fn ConstructionScript)

(fn SetMaterial
  (params (plane :type Static%20Mesh%20Component%20Object%20Reference) (Ability :type Name))
  (switch name Ability
    (:JumpAbility
      (Rendering|Material|SetMaterial plane 0 "/Game/VortexGame/Art/Interface/double_jump_small_Mat.double_jump_small_Mat")
      (return))
    (:MeleeAttackAbility
      (Rendering|Material|SetMaterial plane 0 "/Game/VortexGame/Art/Interface/melee_attack_small_Mat.melee_attack_small_Mat")
      (return))
    (:DoubleJumpAbility
      (Rendering|Material|SetMaterial plane 0 "/Game/VortexGame/Art/Interface/double_jump_small_Mat.double_jump_small_Mat")
      (return))
    (:SprintAbility
      (Rendering|Material|SetMaterial plane 0 "/Game/VortexGame/Art/Interface/dash_small_Mat.dash_small_Mat")
      (return))))

(fn SetAbility
  (params (abilityActivated :type Name))
  (bind _playerref (Variables|Default|GetPlayerRef))
  (bind _asbp_player_side_scroller (Utilities|Casting|CastToBP_PlayerSideScroller (Pawn|GetControlledPawn (Variables|Default|GetPlayerRef))))
  (if (>= (Variables|/Game/VortexGame/Core/BP_PlayerSideScroller.BP_PlayerSideScroller_C|GetMoney _asbp_player_side_scroller) (Variables|Default|GetPrice))
    (Variables|/Game/VortexGame/Core/BP_PlayerSideScroller.BP_PlayerSideScroller_C|SetMoney _asbp_player_side_scroller (- (Variables|/Game/VortexGame/Core/BP_PlayerSideScroller.BP_PlayerSideScroller_C|GetMoney _asbp_player_side_scroller) (Variables|Default|GetPrice)))
    (switch name abilityActivated
      (:JumpAbility
        (Variables|/Game/VortexGame/Core/BP_PlayerController.BP_PlayerController_C|SetJumpAbility _playerref true)
        (Development|PrintString "Gained Jump Ability"))
      (:MeleeAttackAbility
        (Variables|/Game/VortexGame/Core/BP_PlayerController.BP_PlayerController_C|SetMeleeAttackAbility _playerref true)
        (Development|PrintString "Gained attack Ability"))
      (:DoubleJumpAbility
        (Variables|/Game/VortexGame/Core/BP_PlayerController.BP_PlayerController_C|SetDoubleJumpAbility _playerref true)
        (Development|PrintString "Gained double Jump Ability"))
      (:SprintAbility
        (Variables|/Game/VortexGame/Core/BP_PlayerController.BP_PlayerController_C|SetSprintAbility _playerref true)
        (Development|PrintString "Gained sprint Ability")))
    (else
      (Development|PrintString "Not Enough Money"))))
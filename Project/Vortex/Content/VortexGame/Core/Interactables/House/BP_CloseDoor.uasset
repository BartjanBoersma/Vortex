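; House door interactable that swings shut when the side-scroller player enters its box and drives the MetroidVania game mode's round counter.
; Overlap sets a flag that Tick uses to play a yaw timeline.
; On finish it resets its linked door to 90 degrees yaw, and TriggerRound doors increment the round.
; Doors without TriggerRound decrement the round when reset.
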(event OnComponentBeginOverlap(Box)
  (params (OverlappedComponent :type Primitive%20Component%20Object%20Reference) (OtherActor :type Actor%20Object%20Reference) (OtherComp :type Primitive%20Component%20Object%20Reference) (OtherBodyIndex :type Integer) (bFromSweep :type Boolean) (SweepResult :type Hit%20Result%20Structure%20%28by%20ref%29))
  (Utilities|Casting|CastToBP_PlayerSideScroller OtherActor)
  (Variables|Default|Setclose true))

(event Custom|ResetDoor
  (Transformation|SetWorldRotation (Variables|Default|GetScene) "0,90.000000, 0" false false)
  (Variables|Default|Setclosed false)
  (Components|Timeline|SetNewTime (Variables|Default|GetOpenDoor) 0.0)
  (Variables|Default|Setclose false)
  (if (not (Variables|Default|GetTriggerRound))
    (bind _asgm_metroid_vania (Utilities|Casting|CastToGM_MetroidVania (Game|GetGameMode)))
    (Math|Integer|DecrementInt (Variables|/Game/VortexGame/Core/GameModes/GM_MetroidVania.GM_MetroidVania_C|GetRound _asgm_metroid_vania))))

(event EventTick
  (params (DeltaSeconds :type Float%20%28single-precision%29))
  (if (and (Variables|Default|Getclose) (Math|Boolean|NotEqual(Boolean) (Variables|Default|Getclosed) true))
    (bind _rotation (Timeline|OpenDoor Play)
      (:Update
        (Transformation|SetWorldRotation (Variables|Default|GetScene) (Math|Rotator|MakeRotator 0.0 0.0 _rotation) false false))
      (:Finished
        (Variables|Default|Setclosed true)
        (CallFunction|ResetDoor (Variables|Default|GetlinkedDoor))
        (if (Variables|Default|GetTriggerRound)
          (bind _asgm_metroid_vania (Utilities|Casting|CastToGM_MetroidVania (Game|GetGameMode)))
          (bind _result (Math|Integer|IncrementInt (Variables|/Game/VortexGame/Core/GameModes/GM_MetroidVania.GM_MetroidVania_C|GetRound _asgm_metroid_vania))
            (:%20%20
              (Development|PrintString (Utilities|String|ToString(Integer) _result)))))))))

(fn ConstructionScript)
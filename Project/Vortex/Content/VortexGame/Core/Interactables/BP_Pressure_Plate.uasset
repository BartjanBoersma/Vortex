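; BP_Pressure_Plate is an interactable pressure plate that tracks whether something is overlapping its CollisionBox.
; Begin overlap sets IsActive and PlateTrue, end overlap clears both, and each change prints a debug message.
; There is no actor filter or overlap count, so the first overlap end deactivates the plate even if other objects remain on it.
; PlateTrue is only written here, never read.
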(event OnComponentBeginOverlap(CollisionBox)
  (params (OverlappedComponent :type Primitive%20Component%20Object%20Reference) (OtherActor :type Actor%20Object%20Reference) (OtherComp :type Primitive%20Component%20Object%20Reference) (OtherBodyIndex :type Integer) (bFromSweep :type Boolean) (SweepResult :type Hit%20Result%20Structure%20%28by%20ref%29))
  (if true
    (if (not (Variables|Default|GetIsActive))
      (Variables|Default|SetIsActive true)
      (Development|PrintString "Button is now Active")
      (Variables|Default|SetPlate_True true))))

(event OnComponentEndOverlap(CollisionBox)
  (params (OverlappedComponent :type Primitive%20Component%20Object%20Reference) (OtherActor :type Actor%20Object%20Reference) (OtherComp :type Primitive%20Component%20Object%20Reference) (OtherBodyIndex :type Integer))
  (if true
    (if (Variables|Default|GetIsActive)
      (Variables|Default|SetIsActive false)
      (Development|PrintString "Button is now inactive")
      (Variables|Default|SetPlate_True false))))

(fn ConstructionScript)
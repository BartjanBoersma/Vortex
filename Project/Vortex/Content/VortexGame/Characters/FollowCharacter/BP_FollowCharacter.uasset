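; BP_FollowCharacter is a character that trails a side-scroller player along that player's movement spline.
; Overlap begin and end with BP_PlayerSideScroller set and clear the follow target.
; Each Tick compares the target's timeline position with its own, playing the timeline forward when the target is ahead, otherwise reversing, and stopping without a target.
; Timeline updates heavily smooth the alpha by lerp and place the actor at that spline position.
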(event EventBeginPlay)

(event EventTick
  (params (DeltaSeconds :type Float%20%28single-precision%29))
  (bind _followobject (Variables|Default|GetFollowObject))
  (Utilities|IsValid _followobject
    (:Is%20Valid
      (if (> (Components|Timeline|GetPlaybackPosition (Variables|/Game/VortexGame/Core/BP_PlayerSideScroller.BP_PlayerSideScroller_C|GetTimeline_0 _followobject)) (Components|Timeline|GetPlaybackPosition (Variables|Default|GetTimeline_0)))
        (bind _alpha (Timeline|Timeline_0 Play)
          (:Update
            (bind _output_get (Variables|Default|SetCurrentSplinePosition (Math|Float|Lerp _alpha (Variables|Default|GetCurrentSplinePosition) 0.99)))
            (CallFunction|MoveAlongSpline (Variables|/Game/VortexGame/Core/Tools/BP_BasicSpline.BP_BasicSpline_C|GetSpline (Variables|/Game/VortexGame/Core/BP_PlayerSideScroller.BP_PlayerSideScroller_C|GetMovementSpline _followobject)) _output_get self false false)))
        (else
          (Timeline|Timeline_0 Reverse))))
    (:Is%20Not%20Valid
      (Timeline|Timeline_0 Stop))))

(event Collision|EventActorBeginOverlap
  (params (OtherActor :type Actor%20Object%20Reference))
  (bind _asbp_player_side_scroller (Utilities|Casting|CastToBP_PlayerSideScroller OtherActor))
  (Variables|Default|SetFollowObject _asbp_player_side_scroller))

(event Collision|EventActorEndOverlap
  (params (OtherActor :type Actor%20Object%20Reference))
  (Utilities|Casting|CastToBP_PlayerSideScroller OtherActor)
  (Variables|Default|SetFollowObject 0))

(fn ConstructionScript
  (|CallParentFunction))